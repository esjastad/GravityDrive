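; BP_PlayerController is the player controller that switches the player between on-foot character, ship builder and starship flight modes.
; On BeginPlay it caches the player character, finds the ship manager and flight pawn in the level, and creates the build HUD linked to the manager.
; Each Interact press cycles the mode enum and possesses the next pawn, showing the build HUD and mouse cursor only while building.
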(event `self.ReceiveBeginPlay`
  (`|ExecutionSequence`
    (:`then_0`
      (bind _asbp_base_character (cast `/Game/BP_BaseCharacter` (`GameplayStatics.GetPlayerPawn` 0)))
      (set `self.PlayerCharacterReference` _asbp_base_character))
    (:`then_1`
      (bind _outactors (`GameplayStatics.GetAllActorsOfClass` "/Game/ShipBuilder/BP_ShipManager.BP_ShipManager_C"))
      (set `self.ShipManagerReference` (`|GetArrayItem` _outactors)))
    (:`then_2`
      (bind _outactors_2 (`GameplayStatics.GetAllActorsOfClass` "/Game/ShipFlight/BP_ShipFlight.BP_ShipFlight_C"))
      (set `self.StarShipFlightReference` (`|GetArrayItem` _outactors_2)))
    (:`then_3`
      (bind _returnvalue (`|CreateWidget` "/Game/ShipBuilder/BP_ShipBuildWidget.BP_ShipBuildWidget_C" self))
      (bind _output_get (set `self.BuildHud` _returnvalue))
      (`ShipBuildWidget.SetShipReference` _output_get (`self.ShipManagerReference`)))))

(event `InputAction|Interact`
  (params (Key :type "Key Structure"))
  (:`Pressed`
    (switch `/Game/GameComponents/Enum_PawnMode` (`self.PawnModeEnum`)
      (:`NewEnumerator1`
        (set `self.PawnModeEnum` "NewEnumerator2")
        (`self.Possess` (`self.ShipManagerReference`))
        (`UserWidget.AddToViewport` (`self.BuildHud`) 0)
        (set `self.bShowMouseCursor` true))
      (:`NewEnumerator2`
        (set `self.PawnModeEnum` "NewEnumerator3")
        (`Widget.RemoveFromParent` (`self.BuildHud`))
        (`self.Possess` (`self.StarShipFlightReference`))
        (set `self.bShowMouseCursor` false))
      (:`NewEnumerator3`
        (set `self.PawnModeEnum` "NewEnumerator1")
        (`self.Possess` (`self.PlayerCharacterReference`))))))

(fn `UserConstructionScript`)