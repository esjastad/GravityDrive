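; Test actor for a black hole screen-distortion effect on a static mesh that turns to face the player camera every Tick.
; It projects points at plus and minus Radius along its right and up vectors to normalized screen coordinates, feeding them to Mat_BlackHoleDistort as X/Y bounds.
; The dynamic material instance is recreated each Tick, and a debug value prints.
; The Radius-based mesh scaling is disconnected.
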(event `self.ReceiveTick`
  (params (DeltaSeconds :type "Float (single-precision)"))
  (bind (_returnvalue_x _returnvalue_y) (`KismetMathLibrary.BreakVector2D` (`WidgetLayoutLibrary.GetViewportSize`)))
  (bind (_returnvalue_x_2 _returnvalue_y_2) (`KismetMathLibrary.BreakVector2D` (`WidgetLayoutLibrary.GetViewportSize`)))
  (bind _returnvalue (`GameplayStatics.GetPlayerCameraManager` 0))
  (bind _returnvalue_x_3 (`KismetMathLibrary.BreakVector2D` (`WidgetLayoutLibrary.GetViewportSize`)))
  (bind _returnvalue_x_4 (`KismetMathLibrary.BreakVector2D` (`WidgetLayoutLibrary.GetViewportSize`)))
  (bind _returnvalue_2 (/ (`KismetMathLibrary.BreakVector2D` (`GameplayStatics.ProjectWorldToScreen` (`GameplayStatics.GetPlayerController` 0) (+ (`self.K2_GetActorLocation`) (* (`self.GetActorRightVector`) (`self.Radius`))))) _returnvalue_x_3))
  (`|ExecutionSequence`
    (:`then_1`
      (`|ExecutionSequence`
        (:`then_0`
          (`self.K2_SetActorRotation` (`KismetMathLibrary.MakeRotFromXZ` (* (`self.GetActorForwardVector` _returnvalue) -1.0) (`self.GetActorUpVector` _returnvalue)))
          (bind _returnvalue_3 (`PrimitiveComponent.CreateDynamicMaterialInstance` (`self.StaticMesh`) 0 "/Game/SolarBodies/Materials/Mat_BlackHoleDistort.Mat_BlackHoleDistort" "None"))
          (set `self.BlackholeMat` _returnvalue_3))
        (:`then_1`
          (`KismetSystemLibrary.PrintString` (`KismetStringLibrary.Conv_DoubleToString` _returnvalue_2))
          (`MaterialInstanceDynamic.SetScalarParameterValue` (`self.BlackholeMat`) "MinX" _returnvalue_2)
          (`MaterialInstanceDynamic.SetScalarParameterValue` (`self.BlackholeMat`) "MaxX" (/ (`KismetMathLibrary.BreakVector2D` (`GameplayStatics.ProjectWorldToScreen` (`GameplayStatics.GetPlayerController` 0) (- (`self.K2_GetActorLocation`) (* (`self.GetActorRightVector`) (`self.Radius`))))) _returnvalue_x_4)))
        (:`then_2`
          (`MaterialInstanceDynamic.SetScalarParameterValue` (`self.BlackholeMat`) "MinY" (/ (`.Y` (`KismetMathLibrary.BreakVector2D` (`GameplayStatics.ProjectWorldToScreen` (`GameplayStatics.GetPlayerController` 0) (+ (`self.K2_GetActorLocation`) (* (`self.GetActorUpVector`) (`self.Radius`)))))) _returnvalue_y_2))
          (`MaterialInstanceDynamic.SetScalarParameterValue` (`self.BlackholeMat`) "MaxY" (/ (`.Y` (`KismetMathLibrary.BreakVector2D` (`GameplayStatics.ProjectWorldToScreen` (`GameplayStatics.GetPlayerController` 0) (- (`self.K2_GetActorLocation`) (* (`self.GetActorUpVector`) (`self.Radius`)))))) _returnvalue_y)))))))

(fn `UserConstructionScript`)